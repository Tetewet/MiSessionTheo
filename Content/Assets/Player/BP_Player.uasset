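; Player character Blueprint that handles an attack input, damage from snowballs and a weapon switch.
; Pressing the Taper input plays the AM_Taper montage on the mesh.
; Hits from BP_Snowball decrement Life, while hits from BP_HammerTime deactivate the Sword component and activate the Hammer.
; Tick polls Life, which starts at one, and calls the death montage every frame once it reaches zero or below.
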(event EventBeginPlay
  (Variables|Default|SetLife 1.0))

(event Collision|EventActorBeginOverlap
  (params (OtherActor :type Actor%20Object%20Reference)))

(event EventTick
  (params (DeltaSeconds :type Float%20%28single-precision%29))
  (if (<= (Variables|Default|GetLife) 0.0)
    (Animation|PlayAnimMontage "/Game/Assets/Player/AM_Death.AM_Death" 1.0 "None")))

(event Collision|EventHit
  (params (MyComp :type Primitive%20Component%20Object%20Reference) (Other :type Actor%20Object%20Reference) (OtherComp :type Primitive%20Component%20Object%20Reference) (bSelfMoved :type Boolean) (HitLocation :type Vector :default "0, 0, 0") (HitNormal :type Vector :default "0, 0, 0") (NormalImpulse :type Vector :default "0, 0, 0") (Hit :type Hit%20Result%20Structure%20%28by%20ref%29))
  (Utilities|Casting|CastToBP_Snowball Other
    (:then
      (bind _result (Math|Float|DecrementFloat (Variables|Default|GetLife))
        (:%20%20
          (Variables|Default|SetLife _result))))
    (:CastFailed
      (Utilities|Casting|CastToBP_HammerTime Other)
      (Components|Activation|Deactivate (Variables|Default|GetSword))
      (Components|Activation|Activate (Variables|Default|GetHammer) false))))

(event Input|ActionEvents|InputActionTaper
  (params (Key :type Key%20Structure))
  (:Pressed
    (Animation|Montage|PlayMontage (Variables|Character|GetMesh) "/Game/Assets/Player/AM_Taper.AM_Taper")))

(fn ConstructionScript
  (|CallParentFunction))